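; Player pawn for a game with in-game programming, handling movement, look, item interaction and the code-entry menu.
; Axis inputs drive control-rotation-relative movement and camera yaw/pitch, while Interact messages the first overlapping actor implementing InteractInterface.
; OpenCodeMenu flip-flops between a focused CodeInputMenu with cursor and game-only input.
; BeginPlay adds the HUD, but closing the menu calls RemoveAllWidgets, which also removes it.
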(event EventBeginPlay
  ;[1 1 1] Add HUD
  (bind _returnvalue (UserInterface|CreateWidget "/Game/Widgets/HUD.HUD_C" (Game|GetPlayerController 0)))
  (bind _output_get (Variables|Default|SetHudWidget _returnvalue))
  (UserInterface|Viewport|AddtoViewport _output_get 0))

(event Input|ActionEvents|InputActionOpenCodeMenu
  (params (Key :type Key%20Structure))
  (bind _returnvalue (Game|GetPlayerController 0))
  ;[1 1 1] Programming Window
  (:Pressed
    (Utilities|FlowControl|FlipFlop
      (:A
        (Input|SetInputModeUIOnly _returnvalue 0 "DoNotLock")
        (bind _returnvalue_2 (UserInterface|CreateWidget "/Game/Widgets/CodeInputMenu.CodeInputMenu_C" _returnvalue))
        (UserInterface|Viewport|AddtoViewport _returnvalue_2 0)
        (Widget|SetKeyboardFocus _returnvalue_2)
        (Variables|/Script/Engine.PlayerController|SetbShowMouseCursor _returnvalue true))
      (:B
        (Viewport|RemoveAllWidgets)
        (Input|SetInputModeGameOnly _returnvalue)
        (Variables|/Script/Engine.PlayerController|SetbShowMouseCursor _returnvalue false)))))

(event Input|ActionEvents|InputActionInteract
  (params (Key :type Key%20Structure))
  ;[1 1 1] Interact with Item
  (:Pressed
    (bind _array_element (Utilities|Array|ForEachLoopwithBreak (Collision|GetOverlappingActors 0 :!class /Script/Engine.Actor) :!label _label)
      (:LoopBody
        (if (Utilities|DoesObjectImplementInterface _array_element "/Game/InventorySystem/InteractInterface.InteractInterface_C")
          (Class|InteractInterface|Interact(Message) _array_element)
          (goto _label Break))))))

(event Input|AxisEvents|InputAxisRotateSideways
  (params (AxisValue :type Float%20%28single-precision%29))
  ;[1 1 1] Rotation
  (Pawn|Input|AddControllerYawInput AxisValue))

(event Input|AxisEvents|InputAxisForwardBackward
  (params (AxisValue :type Float%20%28single-precision%29))
  ;[1 1 1] Movement
  (Pawn|Input|AddMovementInput (Math|Vector|GetForwardVector (Pawn|GetControlRotation :!class /Script/Engine.Pawn)) AxisValue false))

(event Input|AxisEvents|InputAxisSideways
  (params (AxisValue :type Float%20%28single-precision%29))
  ;[1 1 1] Movement
  (Pawn|Input|AddMovementInput (Math|Vector|GetRightVector (Pawn|GetControlRotation :!class /Script/Engine.Pawn)) AxisValue false))

(event Input|AxisEvents|InputAxisRotateUpDown
  (params (AxisValue :type Float%20%28single-precision%29))
  ;[1 1 1] Rotation
  (Pawn|Input|AddControllerPitchInput AxisValue))

(fn ConstructionScript)